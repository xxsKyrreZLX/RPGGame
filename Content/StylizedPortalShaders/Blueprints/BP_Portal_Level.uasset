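; BP_Portal_Level is a portal actor that sends the player to another level when they step into it.
; When CanTeleport is set, an overlap on its Collision component by an actor tagged "Player" opens the level named by LevelName.
; The construction script applies the configured material and visibility to the portal plane and assigns a texture target to the RC component.
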(event `self.Collision.OnComponentBeginOverlap`
  (params (OverlappedComponent :type "PrimitiveComponent Object Reference") (OtherActor :type "Actor Object Reference") (OtherComp :type "PrimitiveComponent Object Reference") (OtherBodyIndex :type Integer) (bFromSweep :type Boolean) (SweepResult :type "HitResult Structure (by ref)"))
  ;[1 1 1] Teleport to another gate
  (if (`self.canTeleport`)
    (if (`self.ActorHasTag` OtherActor "Player")
      (`GameplayStatics.OpenLevel` (`KismetStringLibrary.Conv_StringToName` (`self.Level Name`))))))

(fn `UserConstructionScript`
  (`PrimitiveComponent.SetMaterial` (`self.SM_Plane`) 0 (`self.Material`))
  (`SceneComponent.SetVisibility` (`self.SM_Plane`) (`self.Portal Visibility`) false)
  (set `SceneCaptureComponentCube.TextureTarget` (`self.Texture Target`) (`self.RC`)))