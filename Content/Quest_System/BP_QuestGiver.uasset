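; BP_QuestGiver is an interactable actor that plays dialogue and then offers its quests to the player.
; A trigger radius shows an interact prompt for BP_ThirdPersonCharacter, rotated every tick to face the camera.
; Each Interact call advances the Dialogue array in a dialogue widget, then opens WB_QuestGiver filled from the Quests array.
; Interacting again or calling CloseWidget removes the quest widget and restores game-only input.
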(event `self.ReceiveTick`
  (params (DeltaSeconds :type "Float (single-precision)"))
  (`SceneComponent.K2_SetWorldRotation` (`self.Interact Widget`) (`KismetMathLibrary.FindLookAtRotation` (`SceneComponent.K2_GetComponentLocation` (`self.Interact Widget`)) (`SceneComponent.K2_GetComponentLocation` (`PlayerCameraManager.TransformComponent` (`GameplayStatics.GetPlayerCameraManager` 0)))) false false))

(event `self.Trigger Radius.OnComponentBeginOverlap`
  (params (OverlappedComponent :type "PrimitiveComponent Object Reference") (OtherActor :type "Actor Object Reference") (OtherComp :type "PrimitiveComponent Object Reference") (OtherBodyIndex :type Integer) (bFromSweep :type Boolean) (SweepResult :type "HitResult Structure (by ref)"))
  ;[1 1 1] Detect Assasination
  (cast `/Game/ThirdPerson/Blueprints/BP_ThirdPersonCharacter` OtherActor)
  (`SceneComponent.SetVisibility` (`self.Interact Widget`) true false))

(event `self.Trigger Radius.OnComponentEndOverlap`
  (params (OverlappedComponent :type "PrimitiveComponent Object Reference") (OtherActor :type "Actor Object Reference") (OtherComp :type "PrimitiveComponent Object Reference") (OtherBodyIndex :type Integer))
  ;[1 1 1] Detect Assasination
  (cast `/Game/ThirdPerson/Blueprints/BP_ThirdPersonCharacter` OtherActor)
  (`SceneComponent.SetVisibility` (`self.Interact Widget`) false false))

(event `/Game/Quest_System/BPI_QuestGiver.Interact`
  (bind _returnvalue (`GameplayStatics.GetPlayerController` 0))
  (bind _returnvalue_2 (`GameplayStatics.GetPlayerController` 0))
  ;[1 1 1] Call Quest Widget
  (if (not (`self.widgetActive`))
    (if (not (`self.DialogueOpen`))
      ;;[1 1 1] Create dialogue
      (bind _returnvalue_3 (`|CreateWidget` "/Game/Quest_System/WB_QuestGiverDialogue.WB_QuestGiverDialogue_C"))
      (bind _output_get (set `self.Dialogue Widget` _returnvalue_3))
      (`UserWidget.AddToViewport` _output_get 0)
      (set `self.DialogueOpen` true)
      (`TextBlock.SetText` (`/Game/Quest_System/WB_QuestGiverDialogue.DialogueText` (`self.Dialogue Widget`)) (`KismetTextLibrary.Conv_StringToText` (`|GetArrayItem` (`self.Dialogue`))))
      (set `PlayerController.bShowMouseCursor` true _returnvalue_2)
      (`WidgetBlueprintLibrary.SetInputMode_GameAndUIEx` _returnvalue_2 (`self.QuestWidget`))
      (else
        ;;[1 1 1] iteratively get dialogue
        (if (>= (`self.DialogueIndex`) (`KismetArrayLibrary.Array_Length` (`self.Dialogue`)))
          (`Widget.RemoveFromParent` (`self.Dialogue Widget`))
          (set `self.Dialogue Widget` null)
          (set `self.DialogueIndex` 1)
          (set `self.DialogueOpen` false)
          (`self.Open Quests Widget`)
          (else
            (`TextBlock.SetText` (`/Game/Quest_System/WB_QuestGiverDialogue.DialogueText` (`self.Dialogue Widget`)) (`KismetTextLibrary.Conv_StringToText` (`|GetArrayItem` (`self.Dialogue`) (`self.DialogueIndex`))))
            (`/Engine/EditorBlueprintResources/StandardMacros.IncrementInt` (`self.DialogueIndex`))))))
    (else
      (`Widget.RemoveFromParent` (`self.QuestWidget`) :!label _label)
      (set `self.QuestWidget` null)
      (set `PlayerController.bShowMouseCursor` false _returnvalue)
      (`WidgetBlueprintLibrary.SetInputMode_GameOnly` _returnvalue)
      (set `self.widgetActive` false))))

(event `Close Widget`
  ;[1 1 1] Call Quest Widget
  (goto _label))

(event `Open Quests Widget`
  ;[1 1 1] Call Quest Widget
  ;;[1 1 1] Open Quest Widget
  (bind _returnvalue (`|CreateWidget` "/Game/Quest_System/WB_QuestGiver.WB_QuestGiver_C"))
  (bind _output_get (set `self.QuestWidget` _returnvalue))
  (`UserWidget.AddToViewport` _output_get 0)
  (set `self.widgetActive` true)
  (set `/Game/Quest_System/WB_QuestGiver.Quest Giver BP` self (`self.QuestWidget`))
  (for _array_element (`self.quests`)
    (`/Game/Quest_System/WB_QuestGiver.Add Quest` (`self.QuestWidget`) _array_element)))

(fn `UserConstructionScript`)