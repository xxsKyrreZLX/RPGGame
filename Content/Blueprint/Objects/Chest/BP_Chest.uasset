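; BP_Chest is an openable chest that rewards the player once with an item and XP.
; OpenChest sets a one-shot flag, plays the open animation, then reports to the player character's quest component and adds XP through its stats component.
; It also allows teleporting on an optional linked portal and returns the chest's Item to the caller.
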(fn `Open Chest`
  (returns (Item :type "/Game/EquipmentSystem/S_Slots Structure"))
  (bind _enableportal (`self.EnablePortal`))
  (if (not (`self.isOpened`))
    (set `self.isOpened` true)
    (`SkeletalMeshComponent.PlayAnimation` (`self.Chest`) "/Game/Blueprint/Objects/Chest/Chest_Open.Chest_Open" false)
    (bind _asbp_third_person_character (cast `/Game/ThirdPerson/Blueprints/BP_ThirdPersonCharacter` (`GameplayStatics.GetPlayerCharacter` 0)))
    (`/Game/Quest_System/BPC_Quest.Open Chest` (`/Game/ThirdPerson/Blueprints/BP_ThirdPersonCharacter.BPC_Quest` _asbp_third_person_character) self)
    (`/Game/Blueprint/BPC_PlayerStats.Increase XP` (`/Game/ThirdPerson/Blueprints/BP_ThirdPersonCharacter.BPC_PlayerStats` _asbp_third_person_character) (`self.Added XP`))
    (if (!= _enableportal null)
      (set `/Game/StylizedPortalShaders/Blueprints/BP_Portal_Level.canTeleport` true _enableportal))
    (return (`self.Item`))))

(fn `UserConstructionScript`)