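; Animal AI Blueprint that chases and melee-attacks the player when its PawnSensing component sees a pawn tagged Player.
; AI MoveTo approaches the first player character, then plays an attack montage guarded by an IsAttacking flag, which clears after a short post-montage delay.
; A montage notify triggers a forward sphere trace, drawn for debugging, that applies AttackDamage to the hit pawn.
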(event `self.PawnSensing.OnSeePawn`
  (params (Pawn :type "Pawn Object Reference"))
  (bind _returnvalue (`self.K2_GetActorLocation`))
  (if (`self.ActorHasTag` Pawn "Player")
    (`|AIMoveTo` self (0.0 0.0 0.0) (`GameplayStatics.GetPlayerCharacter` 0) 100.0
      (:`OnSuccess`
        (if (not (`self.isAttacking`))
          (set `self.isAttacking` true)
          (`|PlayMontage` (`self.Mesh`) (`self.AttackMontage`)
            (:`OnCompleted`
              (`KismetSystemLibrary.Delay` 2.0)
              (set `self.isAttacking` false))
            (:`OnNotifyBegin`
              (bind (_outhit _returnvalue_2) (`KismetSystemLibrary.SphereTraceSingleForObjects` :`Start` _returnvalue :`End` (+ _returnvalue (* (`KismetMathLibrary.GetForwardVector` (`self.K2_GetActorRotation`)) 500.0)) :`Radius` 350.0 :`ObjectTypes` (`|MakeArray` "ObjectTypeQuery3" :!type "EObjectTypeQuery Enum") :`DrawDebugType` "ForDuration"))
              (if _returnvalue_2
                (`GameplayStatics.ApplyDamage` (`.HitActor` (`GameplayStatics.BreakHitResult` _outhit)) (`self.Attack Damage`))))))))))

(fn `UserConstructionScript`
  (`parent.UserConstructionScript`))