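; BP_Dummy is a target character that takes damage and can be stealth-assassinated.
; An overlap radius toggles the assassination prompt; that prompt and the health bar turn toward the camera every tick.
; Damage plays a random hit reaction, launches it along the player's facing and lowers health via BPCPlayerStats, ragdolling on death.
; StealthBackAssasin plays the victim montage, triggers delayed ragdoll and death sound, and returns alignment location and rotation.
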(event `self.ReceiveBeginPlay`
  (bind _aswb_dummy_health_bar (cast `/Game/UI/WB_DummyHealthBar` (`WidgetComponent.GetWidget` (`self.Health Bar Widget`))))
  (set `self.HealthBar UI` _aswb_dummy_health_bar))

(event `self.ReceiveTick`
  (params (DeltaSeconds :type "Float (single-precision)"))
  (`SceneComponent.K2_SetWorldRotation` (`self.WI_Assasinate`) (`KismetMathLibrary.FindLookAtRotation` (`SceneComponent.K2_GetComponentLocation` (`self.WI_Assasinate`)) (`SceneComponent.K2_GetComponentLocation` (`PlayerCameraManager.TransformComponent` (`GameplayStatics.GetPlayerCameraManager` 0)))) false false)
  (`SceneComponent.K2_SetWorldRotation` (`self.Health Bar Widget`) (`KismetMathLibrary.FindLookAtRotation` (`SceneComponent.K2_GetComponentLocation` (`self.WI_Assasinate`)) (`SceneComponent.K2_GetComponentLocation` (`PlayerCameraManager.TransformComponent` (`GameplayStatics.GetPlayerCameraManager` 0)))) false false))

(event `Ragdoll`
  ;[1 1 1] Ragdoll
  (`|ExecutionSequence`
    (:`then_0`
      (`KismetSystemLibrary.Delay` 2.5)
      (`PrimitiveComponent.SetSimulatePhysics` (`self.Mesh`) true))
    (:`then_1`
      (`KismetSystemLibrary.Delay` 0.8)
      (`GameplayStatics.PlaySoundAtLocation` "/Game/Audio/Grunts-Hits/SC_Death.SC_Death" (`self.K2_GetActorLocation`) (struct) 1.0 1.0 0.0 "/Game/Audio/SA_Charactor.SA_Charactor" null null null))))

(event `self.Assasination Radius.OnComponentBeginOverlap`
  (params (OverlappedComponent :type "PrimitiveComponent Object Reference") (OtherActor :type "Actor Object Reference") (OtherComp :type "PrimitiveComponent Object Reference") (OtherBodyIndex :type Integer) (bFromSweep :type Boolean) (SweepResult :type "HitResult Structure (by ref)"))
  ;[1 1 1] Detect Assasination
  (cast `/Game/ThirdPerson/Blueprints/BP_ThirdPersonCharacter` OtherActor)
  (`SceneComponent.SetVisibility` (`self.WI_Assasinate`) true false))

(event `self.Assasination Radius.OnComponentEndOverlap`
  (params (OverlappedComponent :type "PrimitiveComponent Object Reference") (OtherActor :type "Actor Object Reference") (OtherComp :type "PrimitiveComponent Object Reference") (OtherBodyIndex :type Integer))
  ;[1 1 1] Detect Assasination
  (cast `/Game/ThirdPerson/Blueprints/BP_ThirdPersonCharacter` OtherActor)
  (`SceneComponent.SetVisibility` (`self.WI_Assasinate`) false false))

(event `self.ReceiveAnyDamage`
  (params (Damage :type "Float (single-precision)") (DamageType :type "DamageType Object Reference") (InstigatedBy :type "Controller Object Reference") (DamageCauser :type "Actor Object Reference"))
  ;[1 1 1] Hit by Sword
  (`self.PlayAnimMontage` (`|GetArrayItem` (`self.HitAnim`) (`KismetMathLibrary.RandomInteger` (`KismetArrayLibrary.Array_Length` (`self.HitAnim`)))))
  (bind _asbp_third_person_character (cast `/Game/ThirdPerson/Blueprints/BP_ThirdPersonCharacter` (`GameplayStatics.GetPlayerCharacter` 0)))
  (`self.LaunchCharacter` (* (`KismetMathLibrary.GetForwardVector` (`self.K2_GetActorRotation` _asbp_third_person_character)) 600.0))
  (`GameplayStatics.PlaySoundAtLocation` "/Game/Audio/Grunts-Hits/Death2.Death2" (`self.K2_GetActorLocation`) (struct) 1.0 (`KismetMathLibrary.RandomFloatInRange` -3.0 3.0) 0.0 "/Game/Audio/SA_Charactor.SA_Charactor" null null null)
  (bind _isplayerdead (`/Game/Blueprint/BPC_PlayerStats.Decrease Health` (`self.BPC_PlayerStats`) Damage))
  (if _isplayerdead
    (`PrimitiveComponent.SetSimulatePhysics` (`self.Mesh`) true)
    (`GameplayStatics.PlaySoundAtLocation` "/Game/Audio/Grunts-Hits/SC_Death.SC_Death" (`self.K2_GetActorLocation`) (struct) 1.0 1.0 0.0 "/Game/Audio/SA_Charactor.SA_Charactor" null null null)
    (`SceneComponent.SetVisibility` (`self.Health Bar Widget`) false false)))

(fn `Stealth Back Assasin`
  (returns (`REF Location` :type "Vector Structure") (`Assasin Rotation` :type "Rotator Structure"))
  (`self.PlayAnimMontage` "/Game/Characters/Animatiom/Assasination/Paired_Knife_Stealth_KidneyAndNeck_Vic_Montage.Paired_Knife_Stealth_KidneyAndNeck_Vic_Montage")
  (`self.Ragdoll`)
  (`SceneComponent.SetVisibility` (`self.WI_Assasinate`) false false)
  (return (`SceneComponent.K2_GetComponentLocation` (`self.Assasin REF`)) (`self.K2_GetActorRotation`)))

(fn `UserConstructionScript`)