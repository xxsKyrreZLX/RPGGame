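; Player combat component for BP_ThirdPersonCharacter, handling a four-step sword and kick combo plus bow aiming.
; Attack input briefly turns the character toward control rotation and plays montages by AttackIndex, buffering presses made mid-attack for SwordAttackCombo to continue.
; A timer-looped blade sphere trace and a one-shot stab/kick trace damage "Damageable" actors with blood, sound and camera shake.
; Bow input blocks melee, switches rotation mode and shows a crosshair; Q unequips it.
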(event `self.ReceiveTick`
  (params (DeltaSeconds :type "Float (single-precision)"))
  (bind _character_bp (`self.Character BP`))
  (bind _returnvalue (`Actor.K2_GetActorRotation` _character_bp))
  (bind (_returnvalue_roll _returnvalue_pitch _returnvalue_yaw) (`KismetMathLibrary.BreakRotator` (`KismetMathLibrary.RInterpTo` _returnvalue (`Pawn.GetControlRotation` _character_bp) DeltaSeconds 10.0)))
  ;[1 1 1] orientAttack
  (if (`self.orientAttack`)
    (`Actor.K2_SetActorRotation` _character_bp (`KismetMathLibrary.MakeRotator` (.roll _returnvalue) (.pitch _returnvalue) _returnvalue_yaw) false)))

(event `self.ReceiveBeginPlay`
  (bind _asbp_third_person_character (cast `/Game/ThirdPerson/Blueprints/BP_ThirdPersonCharacter` (`self.GetOwner`)))
  (set `self.Character BP` _asbp_third_person_character)
  (set `self.Character Mesh` (`Character.Mesh` _asbp_third_person_character)))

(event `Attack1`
  ;[1 1 1] Combo System
  ;;[1 1 1] Attack1
  (`/Engine/EditorBlueprintResources/StandardMacros.DoOnce` false :!label _label
    (:`Completed`
      (`KismetSystemLibrary.Delay` 0.1)
      (`|PlayMontage` (`self.Character Mesh`) "/Game/Characters/Animatiom/SwordAttacks/Attack1_Montage.Attack1_Montage"
        (:`then`
          (set `self.Attack Index` 1)
          (goto _label :!via `Reset`))))))

(event `EnhancedInput|/Game/ThirdPerson/Input/Actions/IA_Attack`
  (params (ActionValue :type Boolean) (ElapsedSeconds :type "Float (double-precision)") (TriggeredSeconds :type "Float (double-precision)") (InputAction :type "InputAction Object Reference" :default "/Game/ThirdPerson/Input/Actions/IA_Attack.IA_Attack"))
  ;[1 1 1] Combo System
  ;;[1 1 1] Attack Input
  (:`Started`
    (if (`self.Can Attack`)
      (`self.Sword Attack`)
      (set `self.orientAttack` true)
      (`KismetSystemLibrary.Delay` 0.3)
      (set `self.orientAttack` false))))

(event `Attack2`
  ;[1 1 1] Combo System
  ;;[1 1 1] Attack2
  (`/Engine/EditorBlueprintResources/StandardMacros.DoOnce` false :!label _label_2
    (:`Completed`
      (`KismetSystemLibrary.Delay` 0.1)
      (`|PlayMontage` (`self.Character Mesh`) "/Game/Characters/Animatiom/SwordAttacks/Attack2_Montage.Attack2_Montage"
        (:`then`
          (set `self.Attack Index` 2)
          (goto _label_2 :!via `Reset`))))))

(event `Sword Attack`
  ;[1 1 1] Combo System
  ;;[1 1 1] Sword Attack
  (if (`self.Is Attacking`)
    (set `self.Save Attack` true)
    (else
      (set `self.Is Attacking` true)
      (switch `int` (`self.Attack Index`) :!label _label_3
        (:`0`
          (`self.Attack1`))
        (:`1`
          (`self.Attack2`))
        (:`2`
          (`self.Attack3`))
        (:`3`
          (`self.Attack4`))))))

(event `Sword Attack Combo`
  ;[1 1 1] Combo System
  ;;[1 1 1] Combo
  (if (`self.Save Attack`)
    (set `self.Save Attack` false)
    (goto _label_3)
    (else
      (`self.Stop Combo`))))

(event `Attack3`
  ;[1 1 1] Combo System
  ;;[1 1 1] Attack3
  (`/Engine/EditorBlueprintResources/StandardMacros.DoOnce` false :!label _label_4
    (:`Completed`
      (`KismetSystemLibrary.Delay` 0.1)
      (`|PlayMontage` (`self.Character Mesh`) "/Game/Characters/Animatiom/SwordAttacks/Kick_Montage.Kick_Montage"
        (:`then`
          (set `self.Attack Index` 3)
          (goto _label_4 :!via `Reset`))))))

(event `Stop Combo`
  ;[1 1 1] Combo System
  ;;[1 1 1] Stop combo
  (set `self.Is Attacking` false)
  (set `self.Attack Index` 0))

(event `Attack4`
  ;[1 1 1] Combo System
  ;;[1 1 1] Attack4
  (`/Engine/EditorBlueprintResources/StandardMacros.DoOnce` false :!label _label_5
    (:`Completed`
      (`KismetSystemLibrary.Delay` 0.1)
      (`|PlayMontage` (`self.Character Mesh`) "/Game/Characters/Animatiom/SwordAttacks/Attack3_Montage.Attack3_Montage"
        (:`then`
          (set `self.Attack Index` 4)
          (goto _label_5 :!via `Reset`))))))

(event `Start Sword Trace`
  ;[1 1 1] Sword Trace
  (bind _returnvalue (`KismetSystemLibrary.K2_SetTimerDelegate` (delegate `Sword Trace Loop`) 0.001 true))
  (set `self.SwordTraceLoop` _returnvalue))

(event `Sword Trace Loop`
  (bind _character_bp (`self.Character BP`))
  ;[1 1 1] Sword Trace
  (bind (_outhit _returnvalue) (`KismetSystemLibrary.SphereTraceSingle` :`Start` (`SceneComponent.K2_GetComponentLocation` (`/Game/ThirdPerson/Blueprints/BP_ThirdPersonCharacter.Sword Top Point` _character_bp)) :`End` (`SceneComponent.K2_GetComponentLocation` (`/Game/ThirdPerson/Blueprints/BP_ThirdPersonCharacter.Sword Bottom Point` _character_bp)) :`Radius` 12.0 :`TraceChannel` "TraceTypeQuery1" :`DrawDebugType` "ForDuration" :`DrawTime` 0.2))
  (if _returnvalue
    (bind (_bblockinghit _binitialoverlap _time _distance _location _impactpoint _normal _impactnormal _physmat _hitactor) (`GameplayStatics.BreakHitResult` _outhit))
    (if (`Actor.ActorHasTag` _hitactor "Damageable")
      (`/Engine/EditorBlueprintResources/StandardMacros.DoOnce` false :!label _label_6
        (:`Completed`
          (`GameplayStatics.ApplyDamage` _hitactor 20.0)
          (`GameplayStatics.PlayWorldCameraShake` "/Game/Blueprint/BP_SwordHitCameraShake.BP_SwordHitCameraShake_C" _location 0.0 2000.0)
          (`self.Play Sword Hit Sound`)
          (bind _returnvalue_2 (`GameplayStatics.SpawnEmitterAtLocation` "/Game/Realistic_Starter_VFX_Pack_Vol2/Particles/Blood/P_Blood_Splat_Cone.P_Blood_Splat_Cone" _location (`KismetMathLibrary.MakeRotFromXY` _normal _normal) (0.5 0.5 0.5) true "AutoRelease"))
          (`KismetSystemLibrary.Delay` 0.5)
          (`self.K2_DestroyComponent` _returnvalue_2)
          (goto _label_6 :!via `Reset`))))))

(event `Stop Sword Trace`
  ;[1 1 1] Sword Trace
  (`KismetSystemLibrary.K2_ClearAndInvalidateTimerHandle` (`self.SwordTraceLoop`)))

(event `Play Sword Hit Sound`
  ;[1 1 1] Play Sword Hit Sound
  (`GameplayStatics.PlaySoundAtLocation` "/Game/Audio/SwordHits/MS_SwordHit.MS_SwordHit" (`Actor.K2_GetActorLocation` (`self.GetOwner`)) (struct) 1.0 1.0 0.0 "/Game/Audio/SA_Charactor.SA_Charactor" null null null))

(event `Sphere Trace`
  (bind _returnvalue (`SceneComponent.K2_GetComponentLocation` (`/Game/ThirdPerson/Blueprints/BP_ThirdPersonCharacter.Sphere Trace` (`self.Character BP`))))
  ;[1 1 1] Sphere Trace for Stab and Kick
  (bind (_outhit _returnvalue_2) (`KismetSystemLibrary.SphereTraceSingle` :`Start` _returnvalue :`End` _returnvalue :`Radius` 18.0 :`TraceChannel` "TraceTypeQuery1" :`DrawDebugType` "ForDuration" :`DrawTime` 3.0))
  (if _returnvalue_2
    (bind (_bblockinghit _binitialoverlap _time _distance _location _impactpoint _normal _impactnormal _physmat _hitactor) (`GameplayStatics.BreakHitResult` _outhit))
    (if (`Actor.ActorHasTag` _hitactor "Damageable")
      (`GameplayStatics.ApplyDamage` _hitactor 20.0)
      (`GameplayStatics.PlayWorldCameraShake` "/Game/Blueprint/BP_SwordHitCameraShake.BP_SwordHitCameraShake_C" _location 0.0 2000.0)
      (`GameplayStatics.SpawnEmitterAtLocation` "/Game/Realistic_Starter_VFX_Pack_Vol2/Particles/Blood/P_Blood_Splat_Cone.P_Blood_Splat_Cone" _location (`KismetMathLibrary.MakeRotFromXY` _normal _normal) (0.5 0.5 0.5) true "AutoRelease")
      (`self.Play Sword Hit Sound`))))

(event `EnhancedInput|/Game/ThirdPerson/Input/Actions/IA_BowShoot`
  (params (ActionValue :type Boolean) (ElapsedSeconds :type "Float (double-precision)") (TriggeredSeconds :type "Float (double-precision)") (InputAction :type "InputAction Object Reference" :default "/Game/ThirdPerson/Input/Actions/IA_BowShoot.IA_BowShoot"))
  (bind _character_bp (`self.Character BP`))
  (bind _charactermovement (`Character.CharacterMovement` (`self.Character BP`)))
  (bind _charactermovement_2 (`Character.CharacterMovement` _character_bp))
  ;[1 1 1] Right mouse to shoot
  (:`Started`
    (if (`self.gotBow`)
      (set `self.useBow` true)
      (if (`self.useBow`)
        (set `self.Can Attack` false)
        (set `self.isAiming` true)
        (`/Game/ThirdPerson/Blueprints/BP_ThirdPersonCharacter.Equip Bow In Hands` _character_bp)
        (set `CharacterMovementComponent.bUseControllerDesiredRotation` true _charactermovement_2)
        (set `CharacterMovementComponent.bOrientRotationToMovement` false _charactermovement_2)
        (bind _returnvalue (`|CreateWidget` "/Game/UI/WB_Bow_Crosshair.WB_Bow_Crosshair_C"))
        (bind _output_get (set `self.Bow Crosshair  Widget` _returnvalue))
        (`UserWidget.AddToViewport` _output_get 0))))
  (:`Completed`
    (if (`self.gotBow`)
      (if (`self.useBow`)
        (set `self.Can Attack` true)
        (set `self.isAiming` false)
        (set `CharacterMovementComponent.bUseControllerDesiredRotation` false _charactermovement)
        (set `CharacterMovementComponent.bOrientRotationToMovement` true _charactermovement)
        (`KismetSystemLibrary.Delay` 0.2)
        (bind _bow_crosshair__widget (`self.Bow Crosshair  Widget`)
          (:`then`
            (`Widget.RemoveFromParent` _bow_crosshair__widget)
            (set `self.Bow Crosshair  Widget` null))
          (:`else`))))))

(event `Key|Q`
  (params (Key :type "Key Structure"))
  ;[1 1 1] Q cancel aim
  (:`Pressed`
    (if (`self.useBow`)
      (`/Game/ThirdPerson/Blueprints/BP_ThirdPersonCharacter.Unequip Bow In Hands` (`self.Character BP`))
      (set `self.useBow` false))))