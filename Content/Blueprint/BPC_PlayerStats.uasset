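; Stats component shared by the player, training dummy and AI characters, tracking health, stamina, XP and level.
; BeginPlay casts the owner to set a character type, which selects the HUD or health-bar widget that damage updates.
; Healing and max-health changes choose only between player and dummy widgets, while stamina and XP write directly to the player HUD.
; Filling XP triggers level-up, resetting XP, raising stats and playing sound, animation and Niagara effects.
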(event `self.ReceiveBeginPlay`
  (`KismetSystemLibrary.DelayUntilNextTick`)
  (bind _asbp_third_person_character (cast `/Game/ThirdPerson/Blueprints/BP_ThirdPersonCharacter` (`self.GetOwner`))
    (:`then`
      (set `self.BP PlayerCharacter` _asbp_third_person_character)
      (set `self.isPlayer` true)
      ;[1 1 1] If is Player
      (set `self.Character Type` "NewEnumerator0")
      (`ProgressBar.SetPercent` (`/Game/UI/WB_HUD.XpBar` (`/Game/ThirdPerson/Blueprints/BP_ThirdPersonCharacter.HUD Widget` (`self.BP PlayerCharacter`))) (/ (`self.XP`) (`self.Max XP`)))
      (`ProgressBar.SetPercent` (`/Game/UI/WB_HUD.StaminaBar` (`/Game/ThirdPerson/Blueprints/BP_ThirdPersonCharacter.HUD Widget` (`self.BP PlayerCharacter`))) (/ (`self.Current Stamina`) (`self.Max Stamina`))))
    (:`CastFailed`
      (bind _asbp_dummy (cast `/Game/Blueprint/BP_Dummy` (`self.GetOwner`))
        (:`then`
          (set `self.BP Dummy ` _asbp_dummy)
          (set `self.isPlayer` false)
          (set `self.Character Type` "NewEnumerator1"))
        (:`CastFailed`
          (bind _asbp_ai (cast `/Game/AI/BP_AI` (`self.GetOwner`)))
          (set `self.BP AI` _asbp_ai)
          (set `self.Character Type` "NewEnumerator2")))))
  (`ProgressBar.SetPercent` (select `/Game/Blueprint/E_CharacterTypes` (`self.Character Type`) :`NewEnumerator0` (`/Game/UI/WB_HUD.HealthBar` (`/Game/ThirdPerson/Blueprints/BP_ThirdPersonCharacter.HUD Widget` (`self.BP PlayerCharacter`))) :`NewEnumerator1` (`/Game/UI/WB_DummyHealthBar.HealthBar` (`/Game/Blueprint/BP_Dummy.HealthBar UI` (`self.BP Dummy `))) :`NewEnumerator2` (`/Game/UI/WB_DummyHealthBar.HealthBar` (`/Game/AI/BP_AI.HealthBar UI` (`self.BP AI`)))) (/ (`self.Current Health`) (`self.Max Health`)))
  (if (`self.isPlayer`)
    (`TextBlock.SetText` (`/Game/UI/WB_HUD.XPText` (`/Game/ThirdPerson/Blueprints/BP_ThirdPersonCharacter.HUD Widget` (`self.BP PlayerCharacter`))) (`|FormatText` "{Current XP}/{Max XP}" (`self.XP`) (`self.Max XP`)))
    (`TextBlock.SetText` (`/Game/UI/WB_HUD.LevelText` (`/Game/ThirdPerson/Blueprints/BP_ThirdPersonCharacter.HUD Widget` (`self.BP PlayerCharacter`))) (`KismetTextLibrary.Conv_IntToText` (`self.Level`))))
  (if (`self.isPlayer`)
    _))

(fn `Decrease Health`
  (params (Damage :type "Float (double-precision)"))
  (returns (IsPlayerDead :type Boolean))
  (if (not (<= (`self.Current Health`) 0.0))
    (bind _output_get (set `self.Current Health` (- (`self.Current Health`) Damage)))
    (`ProgressBar.SetPercent` (select `/Game/Blueprint/E_CharacterTypes` (`self.Character Type`) :`NewEnumerator0` (`/Game/UI/WB_HUD.HealthBar` (`/Game/ThirdPerson/Blueprints/BP_ThirdPersonCharacter.HUD Widget` (`self.BP PlayerCharacter`))) :`NewEnumerator1` (`/Game/UI/WB_DummyHealthBar.HealthBar` (`/Game/Blueprint/BP_Dummy.HealthBar UI` (`self.BP Dummy `))) :`NewEnumerator2` (`/Game/UI/WB_DummyHealthBar.HealthBar` (`/Game/AI/BP_AI.HealthBar UI` (`self.BP AI`)))) (/ _output_get (`self.Max Health`)))
    (`TextBlock.SetText` (select `/Game/Blueprint/E_CharacterTypes` (`self.Character Type`) :`NewEnumerator0` (`/Game/UI/WB_HUD.HealthText` (`/Game/ThirdPerson/Blueprints/BP_ThirdPersonCharacter.HUD Widget` (`self.BP PlayerCharacter`))) :`NewEnumerator1` (`/Game/UI/WB_DummyHealthBar.HealthText` (`/Game/Blueprint/BP_Dummy.HealthBar UI` (`self.BP Dummy `))) :`NewEnumerator2` (`/Game/UI/WB_DummyHealthBar.HealthText` (`/Game/AI/BP_AI.HealthBar UI` (`self.BP AI`)))) (`KismetTextLibrary.Conv_DoubleToText` (`self.Current Health`) "HalfToEven"))
    (return (<= (`self.Current Health`) 0.0))
    (else
      (return false))))

(fn `Decrease Stamina`
  (params (`Stamina Deplete` :type "Float (double-precision)"))
  (returns (`NO Stamina Left` :type Boolean))
  (if (not (<= (`self.Current Stamina`) 0.0))
    (set `self.Current Stamina` (- (`self.Current Stamina`) `Stamina Deplete`))
    (`ProgressBar.SetPercent` (`/Game/UI/WB_HUD.StaminaBar` (`/Game/ThirdPerson/Blueprints/BP_ThirdPersonCharacter.HUD Widget` (`self.BP PlayerCharacter`))) (/ (`self.Current Stamina`) (`self.Max Stamina`)))
    (return (<= (`self.Current Stamina`) 0.0))
    (else
      (return true))))

(fn `Increase Health`
  (params (`Added Health` :type "Float (double-precision)"))
  (bind _output_get (set `self.Current Health` (+ (`self.Current Health`) `Added Health`)))
  (if (> _output_get (`self.Max Health`))
    (set `self.Current Health` (`self.Max Health`)))
  (`ProgressBar.SetPercent` (select `bool` (`self.isPlayer`) :`false` (`/Game/UI/WB_DummyHealthBar.HealthBar` (`/Game/Blueprint/BP_Dummy.HealthBar UI` (`self.BP Dummy `))) :`true` (`/Game/UI/WB_HUD.HealthBar` (`/Game/ThirdPerson/Blueprints/BP_ThirdPersonCharacter.HUD Widget` (`self.BP PlayerCharacter`)))) (/ (`self.Current Health`) (`self.Max Health`)))
  (`TextBlock.SetText` (select `bool` (`self.isPlayer`) :`false` (`/Game/UI/WB_DummyHealthBar.HealthText` (`/Game/Blueprint/BP_Dummy.HealthBar UI` (`self.BP Dummy `))) :`true` (`/Game/UI/WB_HUD.HealthText` (`/Game/ThirdPerson/Blueprints/BP_ThirdPersonCharacter.HUD Widget` (`self.BP PlayerCharacter`)))) (`KismetTextLibrary.Conv_DoubleToText` (`self.Current Health`) "HalfToEven")))

(fn `Increase Level`
  (params (`Added Level` :type Integer))
  (bind _hud_widget (`/Game/ThirdPerson/Blueprints/BP_ThirdPersonCharacter.HUD Widget` (`self.BP PlayerCharacter`)))
  (set `self.Level` (+ `Added Level` (`self.Level`)))
  (set `self.Max XP` (+ (`self.Max XP`) 150.0))
  (set `self.XP` 0.0)
  (`TextBlock.SetText` (`/Game/UI/WB_HUD.LevelText` (`/Game/ThirdPerson/Blueprints/BP_ThirdPersonCharacter.HUD Widget` (`self.BP PlayerCharacter`))) (`KismetTextLibrary.Conv_IntToText` (`self.Level`)))
  (`GameplayStatics.PlaySound2D` "/Game/Audio/UI/Levelup1.Levelup1" 1.0 1.0 0.0 null null)
  (`/Game/UI/WB_HUD.Play Level Up Animation` _hud_widget)
  (`TextBlock.SetText` (`/Game/UI/WB_HUD.LevelUpAnimationNumber` _hud_widget) (`KismetTextLibrary.Conv_IntToText` (`self.Level`)))
  (`NiagaraFunctionLibrary.SpawnSystemAttached` "/Game/ParticleSystem/CharacterParticle/NS_Levelup.NS_Levelup" (`Character.Mesh` (`self.BP PlayerCharacter`)) "None" (0.0 0.0 0.0) (struct) "KeepRelativeOffset" true true "AutoRelease")
  (`self.Increase Max Health` 20.0)
  (`self.Increase Health` 20.0)
  (`self.Increase Max Stamina` 20.0))

(fn `Increase Max Health`
  (params (`Added Max Health` :type "Float (double-precision)"))
  (set `self.Max Health` (+ (`self.Max Health`) `Added Max Health`))
  (`ProgressBar.SetPercent` (select `bool` (`self.isPlayer`) :`false` (`/Game/UI/WB_DummyHealthBar.HealthBar` (`/Game/Blueprint/BP_Dummy.HealthBar UI` (`self.BP Dummy `))) :`true` (`/Game/UI/WB_HUD.HealthBar` (`/Game/ThirdPerson/Blueprints/BP_ThirdPersonCharacter.HUD Widget` (`self.BP PlayerCharacter`)))) (/ (`self.Current Health`) (`self.Max Health`)))
  (if (`self.isPlayer`)
    _))

(fn `Increase Max Stamina`
  (params (`Added Max Stamina` :type "Float (double-precision)"))
  (bind _output_get (set `self.Max Stamina` (+ (`self.Max Stamina`) `Added Max Stamina`)))
  (set `self.Current Stamina` _output_get)
  (`ProgressBar.SetPercent` (`/Game/UI/WB_HUD.StaminaBar` (`/Game/ThirdPerson/Blueprints/BP_ThirdPersonCharacter.HUD Widget` (`self.BP PlayerCharacter`))) (/ (`self.Current Stamina`) (`self.Max Stamina`))))

(fn `Increase Stamina`
  (params (`Added Stamina` :type "Float (double-precision)"))
  (set `self.Current Stamina` (+ (`self.Current Stamina`) `Added Stamina`))
  (if (> (`self.Current Stamina`) (`self.Max Stamina`))
    (set `self.Current Stamina` (`self.Max Stamina`)))
  (`ProgressBar.SetPercent` (`/Game/UI/WB_HUD.StaminaBar` (`/Game/ThirdPerson/Blueprints/BP_ThirdPersonCharacter.HUD Widget` (`self.BP PlayerCharacter`))) (/ (`self.Current Stamina`) (`self.Max Stamina`))))

(fn `Increase XP`
  (params (`Added XP` :type "Float (double-precision)"))
  (set `self.XP` (+ (`self.XP`) `Added XP`))
  (if (>= (`self.XP`) (`self.Max XP`))
    (`self.Increase Level` 1))
  (`ProgressBar.SetPercent` (`/Game/UI/WB_HUD.XpBar` (`/Game/ThirdPerson/Blueprints/BP_ThirdPersonCharacter.HUD Widget` (`self.BP PlayerCharacter`))) (/ (`self.XP`) (`self.Max XP`)))
  (`TextBlock.SetText` (`/Game/UI/WB_HUD.XPText` (`/Game/ThirdPerson/Blueprints/BP_ThirdPersonCharacter.HUD Widget` (`self.BP PlayerCharacter`))) (`|FormatText` "{Current XP}/{Max XP}" (`self.XP`) (`self.Max XP`))))