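; BP_Arrow is an arrow actor that damages actors tagged Damageable when it overlaps them at high speed.
; On spawn, collision is disabled for a very short delay, then re-enabled.
; The Collision component's begin overlap checks the tag and a minimum velocity, applies ArrowDamage, and prints the hit actor's name.
; A damaging hit then turns off the arrow's collision.
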(event `self.ReceiveBeginPlay`
  (`self.SetActorEnableCollision` false)
  (`KismetSystemLibrary.Delay` 0.015)
  (`self.SetActorEnableCollision` true))

(event `self.Collision.OnComponentBeginOverlap`
  (params (OverlappedComponent :type "PrimitiveComponent Object Reference") (OtherActor :type "Actor Object Reference") (OtherComp :type "PrimitiveComponent Object Reference") (OtherBodyIndex :type Integer) (bFromSweep :type Boolean) (SweepResult :type "HitResult Structure (by ref)"))
  ;[1 1 1] Enemy can damage/speed >6000
  (if (`self.ActorHasTag` OtherActor "Damageable")
    (if (> (`KismetMathLibrary.VSize` (`self.GetVelocity` self)) 6000.0)
      (`GameplayStatics.ApplyDamage` OtherActor (`self.ArrowDamage`))
      (`KismetSystemLibrary.PrintString` (`KismetSystemLibrary.GetObjectName` OtherActor))
      (`self.SetActorEnableCollision` false))))

(fn `UserConstructionScript`)