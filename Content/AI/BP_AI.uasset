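; Enemy AI character with melee combat, stealth assassination victim handling and camera-facing health, assassinate and investigate widgets.
; Attack requests drive a montage combo with buffered input, while a looping-timer sphere trace or one-shot trace damages Damageable-tagged actors.
; Damage triggers hit reaction and knockback unless InmuseShutdown is set; death ragdolls it, crediting player quest and XP.
; StealthBackAssasin plays the victim montage, delays ragdoll and returns the assassin's alignment transform.
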(event `self.ReceiveBeginPlay`
  (bind _aswb_dummy_health_bar (cast `/Game/UI/WB_DummyHealthBar` (`WidgetComponent.GetWidget` (`self.Health Bar Widget`))))
  (set `self.HealthBar UI` _aswb_dummy_health_bar)
  (if (not (`self.canAssasinate`))
    (`SceneComponent.SetVisibility` (`self.WI_Assasinate`) false false)))

(event `self.ReceiveTick`
  (params (DeltaSeconds :type "Float (single-precision)"))
  (`SceneComponent.K2_SetWorldRotation` (`self.WI_Assasinate`) (`KismetMathLibrary.FindLookAtRotation` (`SceneComponent.K2_GetComponentLocation` (`self.WI_Assasinate`)) (`SceneComponent.K2_GetComponentLocation` (`PlayerCameraManager.TransformComponent` (`GameplayStatics.GetPlayerCameraManager` 0)))) false false)
  (`SceneComponent.K2_SetWorldRotation` (`self.Health Bar Widget`) (`KismetMathLibrary.FindLookAtRotation` (`SceneComponent.K2_GetComponentLocation` (`self.WI_Assasinate`)) (`SceneComponent.K2_GetComponentLocation` (`PlayerCameraManager.TransformComponent` (`GameplayStatics.GetPlayerCameraManager` 0)))) false false)
  (`SceneComponent.K2_SetWorldRotation` (`self.Investgate Widget`) (`KismetMathLibrary.FindLookAtRotation` (`SceneComponent.K2_GetComponentLocation` (`self.WI_Assasinate`)) (`SceneComponent.K2_GetComponentLocation` (`PlayerCameraManager.TransformComponent` (`GameplayStatics.GetPlayerCameraManager` 0)))) false false))

(event `Ragdoll`
  ;[1 1 1] Ragdoll
  (`|ExecutionSequence`
    (:`then_0`
      (`KismetSystemLibrary.Delay` 2.5)
      (`PrimitiveComponent.SetSimulatePhysics` (`self.Mesh`) true))
    (:`then_1`
      (`KismetSystemLibrary.Delay` 0.8)
      (`GameplayStatics.PlaySoundAtLocation` "/Game/Audio/Grunts-Hits/SC_Death.SC_Death" (`self.K2_GetActorLocation`) (struct) 1.0 1.0 0.0 "/Game/Audio/SA_Charactor.SA_Charactor" null null null))))

(event `self.Assasination Radius.OnComponentBeginOverlap`
  (params (OverlappedComponent :type "PrimitiveComponent Object Reference") (OtherActor :type "Actor Object Reference") (OtherComp :type "PrimitiveComponent Object Reference") (OtherBodyIndex :type Integer) (bFromSweep :type Boolean) (SweepResult :type "HitResult Structure (by ref)"))
  ;[1 1 1] Detect Assasination
  (if (`self.canAssasinate`)
    (cast `/Game/ThirdPerson/Blueprints/BP_ThirdPersonCharacter` OtherActor)
    (`SceneComponent.SetVisibility` (`self.WI_Assasinate`) true false)))

(event `self.Assasination Radius.OnComponentEndOverlap`
  (params (OverlappedComponent :type "PrimitiveComponent Object Reference") (OtherActor :type "Actor Object Reference") (OtherComp :type "PrimitiveComponent Object Reference") (OtherBodyIndex :type Integer))
  ;[1 1 1] Detect Assasination
  (cast `/Game/ThirdPerson/Blueprints/BP_ThirdPersonCharacter` OtherActor)
  (`SceneComponent.SetVisibility` (`self.WI_Assasinate`) false false))

(event `self.ReceiveAnyDamage`
  (params (Damage :type "Float (single-precision)") (DamageType :type "DamageType Object Reference") (InstigatedBy :type "Controller Object Reference") (DamageCauser :type "Actor Object Reference"))
  ;[1 1 1] Hit by Sword->any damage
  (if (not (`self.isDead`))
    (if (not (`self.InmuseShutdown`))
      ;;[1 1 1] Important
      (`self.Stop Combo`)
      (`self.PlayAnimMontage` (`|GetArrayItem` (`self.HitAnim`) (`KismetMathLibrary.RandomInteger` (`KismetArrayLibrary.Array_Length` (`self.HitAnim`)))))
      (bind _asbp_third_person_character (cast `/Game/ThirdPerson/Blueprints/BP_ThirdPersonCharacter` (`GameplayStatics.GetPlayerCharacter` 0)))
      (`self.LaunchCharacter` (* (`KismetMathLibrary.GetForwardVector` (`self.K2_GetActorRotation` _asbp_third_person_character)) 600.0))
      (`GameplayStatics.PlaySoundAtLocation` "/Game/Audio/Grunts-Hits/Death2.Death2" (`self.K2_GetActorLocation`) (struct) 1.0 (`KismetMathLibrary.RandomFloatInRange` -3.0 3.0) 0.0 "/Game/Audio/SA_Charactor.SA_Charactor" null null null))
    (bind _isplayerdead (`/Game/Blueprint/BPC_PlayerStats.Decrease Health` (`self.BPC_PlayerStats`) Damage))
    (if _isplayerdead
      (`PrimitiveComponent.SetCollisionObjectType` (`self.Mesh`) "ECC_PhysicsBody")
      (`PrimitiveComponent.SetSimulatePhysics` (`self.Mesh`) true)
      (`GameplayStatics.PlaySoundAtLocation` "/Game/Audio/Grunts-Hits/SC_Death.SC_Death" (`self.K2_GetActorLocation`) (struct) 1.0 1.0 0.0 "/Game/Audio/SA_Charactor.SA_Charactor" null null null)
      (`SceneComponent.SetVisibility` (`self.Health Bar Widget`) false false)
      (`CharacterMovementComponent.SetMovementMode` (`self.CharacterMovement`) "MOVE_None" 0)
      (set `self.isDead` true)
      (set `self.Can Attack` false)
      (`/Engine/EditorBlueprintResources/StandardMacros.DoOnce` false
        (:`Completed`
          (bind _asbp_third_person_character_2 (cast `/Game/ThirdPerson/Blueprints/BP_ThirdPersonCharacter` (`GameplayStatics.GetPlayerCharacter` 0)))
          (`/Game/Quest_System/BPC_Quest.Eliminate Enemy` (`/Game/ThirdPerson/Blueprints/BP_ThirdPersonCharacter.BPC_Quest` _asbp_third_person_character_2) self)
          (`/Game/Blueprint/BPC_PlayerStats.Increase XP` (`/Game/ThirdPerson/Blueprints/BP_ThirdPersonCharacter.BPC_PlayerStats` _asbp_third_person_character_2) (`self.Added XP`)))))))

(event `Attack1`
  ;[1 1 1] Combo System
  ;;[1 1 1] Attack1
  (`/Engine/EditorBlueprintResources/StandardMacros.DoOnce` false :!label _label
    (:`Completed`
      (`KismetSystemLibrary.Delay` 0.1)
      (`|PlayMontage` (`self.Mesh`) "/Game/Characters/Animatiom/SwordAttacks/Attack1_Montage.Attack1_Montage" (`self.Attack Animation Speed`)
        (:`then`
          (set `self.Attack Index` 1)
          (goto _label :!via `Reset`))))))

(event `Sword Attack Combo from BT`
  ;[1 1 1] Combo System
  ;;[1 1 1] Attack Input
  (if (`self.Can Attack`)
    (`self.Sword Attack`)))

(event `Attack2`
  ;[1 1 1] Combo System
  ;;[1 1 1] Attack2
  (`/Engine/EditorBlueprintResources/StandardMacros.DoOnce` false :!label _label_2
    (:`Completed`
      (`KismetSystemLibrary.Delay` 0.1)
      (`|PlayMontage` (`self.Mesh`) "/Game/Characters/Animatiom/SwordAttacks/Attack2_Montage.Attack2_Montage" (`self.Attack Animation Speed`)
        (:`then`
          (set `self.Attack Index` 2)
          (goto _label_2 :!via `Reset`))))))

(event `Sword Attack`
  ;[1 1 1] Combo System
  ;;[1 1 1] Sword Attack
  (if (`self.Is Attacking`)
    (set `self.Save Attack` true)
    (else
      (set `self.Is Attacking` true)
      (switch `int` (`self.Attack Index`) :!label _label_3
        (:`0`
          (`self.Attack1`))
        (:`1`
          (`self.Attack2`))
        (:`2`
          (`self.Attack4`))))))

(event `Sword Attack Combo`
  ;[1 1 1] Combo System
  ;;[1 1 1] Combo
  (if (`self.Save Attack`)
    (set `self.Save Attack` false)
    (goto _label_3)
    (else
      (`self.Stop Combo`))))

(event `Attack3`
  ;[1 1 1] Combo System
  ;;[1 1 1] Attack3 NOT IN USE
  (`/Engine/EditorBlueprintResources/StandardMacros.DoOnce` false :!label _label_4
    (:`Completed`
      (`KismetSystemLibrary.Delay` 0.1)
      (`|PlayMontage` (`self.Mesh`) "/Game/Characters/Animatiom/SwordAttacks/Kick_Montage.Kick_Montage" (`self.Attack Animation Speed`)
        (:`then`
          (set `self.Attack Index` 3)
          (goto _label_4 :!via `Reset`))))))

(event `Stop Combo`
  ;[1 1 1] Combo System
  ;;[1 1 1] Stop combo
  (set `self.Is Attacking` false)
  (set `self.Attack Index` 0))

(event `Attack4`
  ;[1 1 1] Combo System
  ;;[1 1 1] Attack4
  (`/Engine/EditorBlueprintResources/StandardMacros.DoOnce` false :!label _label_5
    (:`Completed`
      (`KismetSystemLibrary.Delay` 0.1)
      (`|PlayMontage` (`self.Mesh`) "/Game/Characters/Animatiom/SwordAttacks/Attack3_Montage.Attack3_Montage" (`self.Attack Animation Speed`)
        (:`then`
          (set `self.Attack Index` 4)
          (goto _label_5 :!via `Reset`))))))

(event `Start Sword Trace`
  ;[1 1 1] Sword Trace
  (bind _returnvalue (`KismetSystemLibrary.K2_SetTimerDelegate` (delegate `Sword Trace Loop`) 0.001 true))
  (set `self.SwordTraceLoop` _returnvalue))

(event `Sword Trace Loop`
  ;[1 1 1] Sword Trace
  (bind (_outhit _returnvalue) (`KismetSystemLibrary.SphereTraceSingle` :`Start` (`SceneComponent.K2_GetComponentLocation` (`self.Sword Top Point`)) :`End` (`SceneComponent.K2_GetComponentLocation` (`self.Sword Bottom Point`)) :`Radius` 12.0 :`TraceChannel` "TraceTypeQuery1" :`DrawDebugType` "ForDuration" :`DrawTime` 0.2))
  (if _returnvalue
    (bind (_bblockinghit _binitialoverlap _time _distance _location _impactpoint _normal _impactnormal _physmat _hitactor) (`GameplayStatics.BreakHitResult` _outhit))
    (if (`self.ActorHasTag` _hitactor "Damageable")
      (`/Engine/EditorBlueprintResources/StandardMacros.DoOnce` false :!label _label_6
        (:`Completed`
          (`GameplayStatics.ApplyDamage` _hitactor 20.0)
          (`GameplayStatics.PlayWorldCameraShake` "/Game/Blueprint/BP_SwordHitCameraShake.BP_SwordHitCameraShake_C" _location 0.0 2000.0)
          (`self.Play Sword Hit Sound`)
          (bind _returnvalue_2 (`GameplayStatics.SpawnEmitterAtLocation` "/Game/Realistic_Starter_VFX_Pack_Vol2/Particles/Blood/P_Blood_Splat_Cone.P_Blood_Splat_Cone" _location (`KismetMathLibrary.MakeRotFromXY` _normal _normal) (0.5 0.5 0.5) true "AutoRelease"))
          (`KismetSystemLibrary.Delay` 0.5)
          ;;[1 1 1] What I deleted?
          (`ActorComponent.K2_DestroyComponent` _returnvalue_2)
          (goto _label_6 :!via `Reset`))))))

(event `Stop Sword Trace`
  ;[1 1 1] Sword Trace
  (`KismetSystemLibrary.K2_ClearAndInvalidateTimerHandle` (`self.SwordTraceLoop`)))

(event `Play Sword Hit Sound`
  ;[1 1 1] Play Sword Hit Sound
  (`GameplayStatics.PlaySoundAtLocation` "/Game/Audio/SwordHits/MS_SwordHit.MS_SwordHit" (`self.K2_GetActorLocation` (`self.GetOwner`)) (struct) 1.0 1.0 0.0 "/Game/Audio/SA_Charactor.SA_Charactor" null null null))

(event `Sphere Trace`
  (bind _returnvalue (`SceneComponent.K2_GetComponentLocation` (`self.SphereTrace`)))
  ;[1 1 1] Sphere Trace for Stab and Kick
  (bind (_outhit _returnvalue_2) (`KismetSystemLibrary.SphereTraceSingle` :`Start` _returnvalue :`End` _returnvalue :`Radius` 40.0 :`TraceChannel` "TraceTypeQuery1" :`DrawDebugType` "ForDuration" :`DrawTime` 3.0))
  (if _returnvalue_2
    (bind (_bblockinghit _binitialoverlap _time _distance _location _impactpoint _normal _impactnormal _physmat _hitactor) (`GameplayStatics.BreakHitResult` _outhit))
    (if (`self.ActorHasTag` _hitactor "Damageable")
      (`GameplayStatics.ApplyDamage` _hitactor 20.0)
      (`GameplayStatics.PlayWorldCameraShake` "/Game/Blueprint/BP_SwordHitCameraShake.BP_SwordHitCameraShake_C" _location 0.0 2000.0)
      (`GameplayStatics.SpawnEmitterAtLocation` "/Game/Realistic_Starter_VFX_Pack_Vol2/Particles/Blood/P_Blood_Splat_Cone.P_Blood_Splat_Cone" _location (`KismetMathLibrary.MakeRotFromXY` _normal _normal) (0.5 0.5 0.5) true "AutoRelease")
      (`self.Play Sword Hit Sound`))))

(event `Investigation Icon`
  (bind _investgate_widget (`self.Investgate Widget`))
  ;[1 1 1] Investigation Icon
  (`/Engine/EditorBlueprintResources/StandardMacros.FlipFlop`
    (:`A`
      (`SceneComponent.SetVisibility` _investgate_widget true false))
    (:`B`
      (`SceneComponent.SetVisibility` _investgate_widget false false))))

(fn `Attack`
  (returns (`Animation Duration` :type "Float (double-precision)"))
  (`self.Sword Attack Combo from BT`)
  (return 0.4))

(fn `Stealth Back Assasin`
  (returns (`REF Location` :type "Vector Structure") (`Assasin Rotation` :type "Rotator Structure"))
  (if (not (`self.isDead`))
    (set `self.isDead` true)
    (`self.PlayAnimMontage` "/Game/Characters/Animatiom/Assasination/Paired_Knife_Stealth_KidneyAndNeck_Vic_Montage.Paired_Knife_Stealth_KidneyAndNeck_Vic_Montage")
    (`self.Ragdoll`)
    (`SceneComponent.SetVisibility` (`self.WI_Assasinate`) false false)
    (`SceneComponent.SetVisibility` (`self.Health Bar Widget`) false false)
    (`CharacterMovementComponent.SetMovementMode` (`self.CharacterMovement`) "MOVE_None" 0)
    (return (`SceneComponent.K2_GetComponentLocation` (`self.Assasin REF`)) (`self.K2_GetActorRotation`))))

(fn `UserConstructionScript`)