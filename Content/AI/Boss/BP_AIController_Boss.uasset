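; Boss AI controller that runs the boss behavior tree and manages the on-screen boss health bar during combat.
; BeginPlay starts BT_AI_Boss, while custom events activate and deactivate boss combat by creating or removing the WB_BossHealthBar widget.
; While that widget is valid, Tick polls Health over MaxHealth and writes the ratio to its progress bar.
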(event `self.ReceiveBeginPlay`
  (`self.RunBehaviorTree` "/Game/AI/Boss/BT_AI_Boss.BT_AI_Boss"))

(event `Activate Boss Combat`
  (bind _returnvalue (`|CreateWidget` "/Game/UI/WB_BossHealthBar.WB_BossHealthBar_C"))
  (bind _output_get (set `self.Boss Health Bar` _returnvalue))
  (`UserWidget.AddToViewport` _returnvalue 0)
  (`UserWidget.AddToViewport` _output_get 0))

(event `Deactivate Boss Combat`
  (bind _boss_health_bar (`self.Boss Health Bar`)
    (:`then`
      (`Widget.RemoveFromParent` _boss_health_bar)
      (set `self.Boss Health Bar` null))
    (:`else`)))

(event `self.ReceiveTick`
  (params (DeltaSeconds :type "Float (single-precision)"))
  (bind _boss_health_bar (`self.Boss Health Bar`)
    (:`then`
      (`ProgressBar.SetPercent` (`/Game/UI/WB_BossHealthBar.HealthBar` _boss_health_bar) (/ (`self.health`) (`self.maxHealth`))))
    (:`else`)))

(fn `UserConstructionScript`
  (`parent.UserConstructionScript`))